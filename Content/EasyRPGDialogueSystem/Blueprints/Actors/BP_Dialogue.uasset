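; BP_Dialogue is a dialogue actor that runs NPC conversations and cutscenes for the EasyRPG dialogue system.
; It creates Widget_Dialogue and steps through main or choice-response entries, playing each line's voice-over and talk montage.
; Cutscenes start at level start or on sphere overlap, with a polling loop pausing the Level Sequence while dialogue shows.
; Outside sequences, the parent NPC can smoothly turn toward the player and back afterward.
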(event OnComponentBeginOverlap(Sphere)
  (params (OverlappedComponent :type Primitive%20Component%20Object%20Reference) (OtherActor :type Actor%20Object%20Reference) (OtherComp :type Primitive%20Component%20Object%20Reference) (OtherBodyIndex :type Integer) (bFromSweep :type Boolean) (SweepResult :type Hit%20Result%20Structure%20%28by%20ref%29))
  ;[0.2135 0.2135 0.2135] Plays cutscene on collision with the sphere collision component. Set the is cutscene variable to false to disable this.
  (if (and (Variables|CutsceneConditions|GetIs%20Cutscene?) (not (Variables|CutsceneConditions|GetAt%20Level%20Start?)))
    (Utilities|FlowControl|DoOnce false
      (:Completed
        (CallFunction|StartCutscene)))))

(event Custom|Show%20Choices%20Box
  (bind _dialogue_widget (Variables|Components|GetDialogue%20Widget))
  ;[0.2135 0.2135 0.2135] Show choices box
  (if (Utilities|Enum|Equal(Enum) (.Line (Utilities|Struct|BreakStruct_DialogueEntry (Variables|/Game/EasyRPGDialogueSystem/Blueprints/Widgets/Widget_Dialogue.Widget_Dialogue_C|GetCurrent%20Dialogue%20Entry _dialogue_widget))) (Utilities|Text|ToText(String) (Variables|/Game/EasyRPGDialogueSystem/Blueprints/Widgets/Widget_Dialogue.Widget_Dialogue_C|GetDialogue%20Final%20Text _dialogue_widget))) :!label _label
    (Widget|SetVisibility (Variables|/Game/EasyRPGDialogueSystem/Blueprints/Widgets/Widget_Dialogue.Widget_Dialogue_C|GetChoicesBox (Variables|Components|GetDialogue%20Widget)) "Visible")
    (Variables|/Script/Engine.PlayerController|SetbShowMouseCursor (Game|GetPlayerController 0) true)
    (else
      (Utilities|FlowControl|Delay 0.1)
      (goto _label))))

(event Custom|Play/Pause%20Cutscene
  ;[0.2135 0.2135 0.2135] Play and pause already existing cutscene sequence.
  (bind _asbp_first_person_character (Utilities|Casting|CastToBP_FirstPersonCharacter (Game|GetPlayerCharacter 0)))
  (Variables|/Game/FirstPerson/Blueprints/BP_FirstPersonCharacter.BP_FirstPersonCharacter_C|SetCurrent%20Dialogue _asbp_first_person_character self)
  (Variables|/Game/FirstPerson/Blueprints/BP_FirstPersonCharacter.BP_FirstPersonCharacter_C|SetIn%20Dialogue _asbp_first_person_character true)
  (if (Variables|CutsceneConditions|GetPause?) :!label _label
    (Utilities|FlowControl|Sequence
      (:then_0
        (Utilities|FlowControl|DoOnce false :!label _label_2
          (:Completed
            (Utilities|IsValid (Variables|/Game/FirstPerson/Blueprints/BP_FirstPersonCharacter.BP_FirstPersonCharacter_C|GetCurrent%20Sequence%20Player _asbp_first_person_character)
              (:Is%20Valid
                (Sequencer|Player|Pause (Variables|/Game/FirstPerson/Blueprints/BP_FirstPersonCharacter.BP_FirstPersonCharacter_C|GetCurrent%20Sequence%20Player _asbp_first_person_character))
                (goto _label_3 Reset))))))
      (:then_1
        _))
    (else
      (Utilities|FlowControl|Sequence
        (:then_0
          (Utilities|FlowControl|DoOnce false :!label _label_3
            (:Completed
              (Utilities|IsValid (Variables|/Game/FirstPerson/Blueprints/BP_FirstPersonCharacter.BP_FirstPersonCharacter_C|GetCurrent%20Sequence%20Player _asbp_first_person_character)
                (:Is%20Valid
                  (Sequencer|Player|Play (Variables|/Game/FirstPerson/Blueprints/BP_FirstPersonCharacter.BP_FirstPersonCharacter_C|GetCurrent%20Sequence%20Player _asbp_first_person_character) :!class /Script/MovieScene.MovieSceneSequencePlayer)
                  (goto _label_2 Reset))))))
        (:then_1
          _))))
  (Utilities|FlowControl|Delay 0.1)
  (goto _label))

(event Custom|Start%20Cutscene
  ;[0.2135 0.2135 0.2135] Starts cutscene for first dialogue actor in cutscene.
  (bind _asbp_first_person_character (Utilities|Casting|CastToBP_FirstPersonCharacter (Game|GetPlayerCharacter 0)))
  (Variables|/Game/FirstPerson/Blueprints/BP_FirstPersonCharacter.BP_FirstPersonCharacter_C|SetCurrent%20Dialogue _asbp_first_person_character self)
  (Variables|/Game/FirstPerson/Blueprints/BP_FirstPersonCharacter.BP_FirstPersonCharacter_C|SetIn%20Dialogue _asbp_first_person_character true)
  (bind _returnvalue (Sequencer|Player|CreateLevelSequencePlayer (Variables|CutsceneReferences|GetLevel%20Sequence)))
  (bind _output_get (Variables|CutsceneReferences|SetSequence%20Player _returnvalue))
  (Variables|/Game/FirstPerson/Blueprints/BP_FirstPersonCharacter.BP_FirstPersonCharacter_C|SetCurrent%20Sequence%20Player _asbp_first_person_character _output_get)
  (if (Variables|CutsceneConditions|GetPause?) :!label _label
    (Utilities|FlowControl|Sequence
      (:then_0
        (Utilities|FlowControl|DoOnce false :!label _label_2
          (:Completed
            (Utilities|IsValid (Variables|CutsceneReferences|GetSequence%20Player)
              (:Is%20Valid
                (Sequencer|Player|Pause (Variables|CutsceneReferences|GetSequence%20Player))
                (goto _label_3 Reset))))))
      (:then_1
        _))
    (else
      (Utilities|FlowControl|Sequence
        (:then_0
          (Utilities|FlowControl|DoOnce false :!label _label_3
            (:Completed
              (Utilities|IsValid (Variables|CutsceneReferences|GetSequence%20Player)
                (:Is%20Valid
                  (Sequencer|Player|Play (Variables|CutsceneReferences|GetSequence%20Player) :!class /Script/MovieScene.MovieSceneSequencePlayer)
                  (goto _label_2 Reset))))))
        (:then_1
          _))))
  (Utilities|FlowControl|Delay 0.1)
  (if (== (Variables|/Game/FirstPerson/Blueprints/BP_FirstPersonCharacter.BP_FirstPersonCharacter_C|GetCurrent%20Dialogue _asbp_first_person_character) self)
    (goto _label)))

(event Custom|End%20Cutscene
  ;[0.2135 0.2135 0.2135] End cutscene. This MUST be activated at the end of each sequence from the last dialogue actor in that sequence. To reenable player movement
  (bind _asbp_first_person_character (Utilities|Casting|CastToBP_FirstPersonCharacter (Game|GetPlayerCharacter 0)))
  (Variables|/Game/FirstPerson/Blueprints/BP_FirstPersonCharacter.BP_FirstPersonCharacter_C|SetCurrent%20Sequence%20Player _asbp_first_person_character 0))

(event Custom|Play%20talk%20animation
  ;[0.2135 0.2135 0.2135] Play talk animation
  (bind _parentnpc (Variables|NPC|GetParentNPC)
    (:then
      (bind _dialogue_widget (Variables|Components|GetDialogue%20Widget)
        (:then
          (Utilities|IsValid (Utilities|Struct|BreakStruct_DialogueEntry (Variables|/Game/EasyRPGDialogueSystem/Blueprints/Widgets/Widget_Dialogue.Widget_Dialogue_C|GetCurrent%20Dialogue%20Entry _dialogue_widget))
            (:Is%20Valid
              (Animation|Montage|PlayMontage (Variables|/Script/Engine.Character|GetMesh _parentnpc) (Utilities|Struct|BreakStruct_DialogueEntry (Variables|/Game/EasyRPGDialogueSystem/Blueprints/Widgets/Widget_Dialogue.Widget_Dialogue_C|GetCurrent%20Dialogue%20Entry _dialogue_widget)) 1.0 0.0 "root"))))
        (:else)))
    (:else)))

(event Custom|Rotate%20to%20player
  (bind _returnvalue (Transformation|GetActorLocation))
  (bind _player_actor (Variables|NPC|GetPlayer%20Actor))
  (bind _parentnpc (Variables|NPC|GetParentNPC))
  (bind _returnvalue_2 (Transformation|GetActorLocation _player_actor))
  (bind _returnvalue_3 (Transformation|GetActorRotation _parentnpc))
  (bind _returnvalue_4 (Math|Rotator|FindLookatRotation _returnvalue _returnvalue_2))
  ;[0.2135 0.2135 0.2135] Rotate NPC to player character
  (if (Variables|NPC|GetNPC%20Rotates)
    (Variables|CutsceneReferences|GetSequence%20Player
      (:then)
      (:else
        (Variables|CutsceneReferences|GetLevel%20Sequence
          (:then)
          (:else
            (bind _parentnpc_2 (Variables|NPC|GetParentNPC)
              (:then
                (Variables|NPC|SetOriginal%20NPC%20Rotation (Transformation|GetActorRotation _parentnpc_2))
                (if (not (Math|Boolean|ANDBoolean (Utilities|Operators|EqualEqual _returnvalue_3 _returnvalue_4 1.0) (Utilities|IsValid (Variables|NPC|GetPlayer%20Actor)) (Utilities|IsValid (Variables|NPC|GetParentNPC)))) :!label _label
                  (Transformation|SetActorRotation (Variables|NPC|GetParentNPC) (Math|Interpolation|RInterpTo _returnvalue_3 _returnvalue_4 (Utilities|Time|GetWorldDeltaSeconds) (Variables|NPC|GetNPC%20Rotation%20Speed)))
                  (Utilities|FlowControl|Delay 0.0)
                  (goto _label)))
              (:else))))))))

(event Custom|Revert%20rotation
  (bind _parentnpc (Variables|NPC|GetParentNPC))
  (bind _original_npc_rotation (Variables|NPC|GetOriginal%20NPC%20Rotation))
  (bind _returnvalue (Transformation|GetActorRotation _parentnpc))
  ;[0.2135 0.2135 0.2135] Revert NPC to original rotation
  (if (Variables|NPC|GetNPC%20Rotates)
    (Variables|CutsceneReferences|GetSequence%20Player
      (:then)
      (:else
        (Variables|CutsceneReferences|GetLevel%20Sequence
          (:then)
          (:else
            (Variables|NPC|GetParentNPC
              (:then
                (if (not (and (Utilities|Operators|EqualEqual _returnvalue _original_npc_rotation 1.0) (Utilities|IsValid (Variables|NPC|GetParentNPC)))) :!label _label
                  (Transformation|SetActorRotation (Variables|NPC|GetParentNPC) (Math|Interpolation|RInterpTo _returnvalue _original_npc_rotation (Utilities|Time|GetWorldDeltaSeconds) (Variables|NPC|GetNPC%20Rotation%20Speed)))
                  (Utilities|FlowControl|Delay 0.0)
                  (goto _label)))
              (:else))))))))

(event EventBeginPlay
  ;[0.2135 0.2135 0.2135] Play cutscene if this dialogue contains the cutscene that plays when the level starts.
  ; Be sure to keep sphere collision component out of the player's reach to avoid retriggering the cutscene.
  ; (WARNING: Do not enable At Level Start for more than one dialogue actor in each level.)
  (if (Variables|CutsceneConditions|GetAt%20Level%20Start?)
    (Utilities|FlowControl|DoOnce false
      (:Completed
        (CallFunction|StartCutscene)))))

(fn ConstructionScript)

(fn AddDialogueWidget
  (params (Player%20Actor :type Actor%20Object%20Reference))
  ;[0.2135 0.2135 0.2135] Create dialogue widget and set variables to pause current cutscene.
  (Utilities|IsValid Player%20Actor
    (:Is%20Valid
      (Variables|NPC|SetPlayer%20Actor Player%20Actor))
    (:Is%20Not%20Valid
      _))
  (bind _returnvalue (UserInterface|CreateWidget "/Game/EasyRPGDialogueSystem/Blueprints/Widgets/Widget_Dialogue.Widget_Dialogue_C" 0 self))
  (bind _output_get (Variables|Components|SetDialogue%20Widget _returnvalue))
  (UserInterface|Viewport|AddtoViewport _output_get 0)
  (Variables|CutsceneConditions|SetFinished? false)
  (Variables|CutsceneConditions|SetPause? true)
  (Variables|Indexes|SetIndex 0)
  ;[0.2135 0.2135 0.2135] Play voice over based on dialogue line.
  (bind _returnvalue_2 (Audio|SpawnSound2D (.VoiceOver (Utilities|Struct|BreakStruct_DialogueEntry (Utilities|Array|Get(acopy) (Utilities|Select :Index (Variables|Indexes|GetDisplayed%20Dialogue%20Index) :Option%200 (Variables|Dialogue|GetDialogueEntries) :Option%201 (Variables|Choices|GetChoice%2001%20Response) :Option%202 (Variables|Choices|GetChoice%2002%20Response))))) 1.0 1.0 0.0 0))
  (Variables|Default|SetCurrentSound _returnvalue_2)
  ;[0.2135 0.2135 0.2135] Pause already existing cutscene when widget is added.
  (if (Variables|CutsceneConditions|GetIs%20Cutscene?)
    (CallFunction|Play/PauseCutscene))
  (Variables|/Game/EasyRPGDialogueSystem/Blueprints/Widgets/Widget_Dialogue.Widget_Dialogue_C|SetCurrent%20Dialogue%20Entry (Variables|Components|GetDialogue%20Widget) (Utilities|Array|Get(acopy) (Utilities|Select :Index (Variables|Indexes|GetDisplayed%20Dialogue%20Index) :Option%200 (Variables|Dialogue|GetDialogueEntries) :Option%201 (Variables|Choices|GetChoice%2001%20Response) :Option%202 (Variables|Choices|GetChoice%2002%20Response)) (Variables|Indexes|GetIndex)))
  (CallFunction|PlayTalkAnimation)
  (CallFunction|RotatetoPlayer))

(fn NextDialogueLine
  (bind _dialogueentries (Variables|Dialogue|GetDialogueEntries))
  (bind _displayed_dialogue_index (Variables|Indexes|GetDisplayed%20Dialogue%20Index))
  (bind _choice_01_response (Variables|Choices|GetChoice%2001%20Response))
  (bind _choice_02_response (Variables|Choices|GetChoice%2002%20Response))
  (bind _index (Variables|Indexes|GetIndex))
  (bind _returnvalue (Utilities|Select :Index _displayed_dialogue_index :Option%200 _dialogueentries :Option%201 _choice_01_response :Option%202 _choice_02_response))
  (bind _output (Utilities|Array|Get(acopy) _returnvalue _index))
  (if (not (Widget|IsVisible (Variables|/Game/EasyRPGDialogueSystem/Blueprints/Widgets/Widget_Dialogue.Widget_Dialogue_C|GetChoicesBox (Variables|Components|GetDialogue%20Widget))))
    ;[0.2135 0.2135 0.2135] Check if current index is less than available length in the Dialogue Entries Array.
    (if (< (Variables|Indexes|GetIndex) (Utilities|Array|Length (Utilities|Select :Index (Variables|Indexes|GetDisplayed%20Dialogue%20Index) :Option%200 (Variables|Dialogue|GetDialogueEntries) :Option%201 (Variables|Choices|GetChoice%2001%20Response) :Option%202 (Variables|Choices|GetChoice%2002%20Response))))
      ;[0.2135 0.2135 0.2135] Increment index and check array length again.
      (Math|Integer|IncrementInt (Variables|Indexes|GetIndex)
        (:%20%20
          (if (< (Variables|Indexes|GetIndex) (Utilities|Array|Length (Utilities|Select :Index (Variables|Indexes|GetDisplayed%20Dialogue%20Index) :Option%200 (Variables|Dialogue|GetDialogueEntries) :Option%201 (Variables|Choices|GetChoice%2001%20Response) :Option%202 (Variables|Choices|GetChoice%2002%20Response))))
            ;[0.2135 0.2135 0.2135] Stop current voice over sound and play the right one based on the current dialogue entry.
            (bind _dialogue_widget (Variables|Components|GetDialogue%20Widget)
              (:then
                (Variables|/Game/EasyRPGDialogueSystem/Blueprints/Widgets/Widget_Dialogue.Widget_Dialogue_C|SetCurrent%20Dialogue%20Entry _dialogue_widget _output)
                (CallFunction|PlayTalkAnimation)
                (bind _currentsound (Variables|Default|GetCurrentSound)
                  (:then
                    (Audio|Components|Audio|Stop _currentsound))
                  (:else
                    _))
                (bind _returnvalue_2 (Audio|SpawnSound2D (.VoiceOver (Utilities|Struct|BreakStruct_DialogueEntry _output)) 1.0 1.0 0.0 0))
                (Variables|Default|SetCurrentSound _returnvalue_2)
                (bind _choice_sound (Variables|/Game/EasyRPGDialogueSystem/Blueprints/Widgets/Widget_Dialogue.Widget_Dialogue_C|GetChoice%20Sound _dialogue_widget)
                  (:then
                    (Audio|Components|Audio|Stop _choice_sound))
                  (:else)))
              (:else))
            (else
              ;[0.2135 0.2135 0.2135] Remove dialogue widget if Index surpassed length.
              (if (not (Math|Boolean|ANDBoolean (== (Variables|Indexes|GetIndex) (Utilities|Array|Length (Variables|Dialogue|GetDialogueEntries))) (Variables|Choices|GetContains%20Choice) (== (Variables|Indexes|GetDisplayed%20Dialogue%20Index) 0)))
                (CallFunction|RemoveDialogue)
                (CallFunction|RevertRotation)))))))))

(fn RemoveDialogue
  (bind _currentsound (Variables|Default|GetCurrentSound))
  ;[1 1 1] Remove dialogue widget and return index
  (bind _dialogue_widget (Variables|Components|GetDialogue%20Widget)
    (:then
      (Widget|RemovefromParent _dialogue_widget)
      (Variables|CutsceneConditions|SetPause? false)
      (Variables|CutsceneConditions|SetFinished? true)
      (Utilities|IsValid _currentsound
        (:Is%20Valid
          (Audio|Components|Audio|Stop _currentsound))
        (:Is%20Not%20Valid
          _))
      (if (Variables|Choices|GetChoicesLoop)
        (Variables|Indexes|SetIndex 0)
        (Variables|Indexes|SetDisplayed%20Dialogue%20Index 0)))
    (:else)))