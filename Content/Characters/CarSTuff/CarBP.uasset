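; CarBP is a car that drives along the path of the first SplinePathBP found in the level, starting at BeginPlay.
; A timeline, with play rate scaled by TimeToComplete, interpolates distance along the spline and sets the car's location and rotation each update.
; On hitting a BP_NPC, it swaps collision from the capsule to the mesh and hides the NPC's talk notification widget.
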(event Custom|MoveObject
  (bind _splineref (Variables|Default|GetSplineRef))
  (bind _spline (Variables|/Game/Characters/CarSTuff/SplinePathBP.SplinePathBP_C|GetSpline _splineref))
  (Components|Timeline|SetPlayRate (Variables|Default|GetMove%20Object%20T) (/ 1.0 (Variables|Default|GetTimeToComplete)))
  (bind _move_track (Timeline|Move%20Object%20T Play)
    (:Update
      (Transformation|SetActorTransform (Math|Transform|MakeTransform (Spline|GetLocationatDistanceAlongSpline _spline (Math|Float|Lerp 0.0 (Spline|GetSplineLength (Variables|/Game/Characters/CarSTuff/SplinePathBP.SplinePathBP_C|GetSpline (Variables|Default|GetSplineRef))) _move_track) "World") (Spline|GetRotationatDistanceAlongSpline _spline (Math|Float|Lerp 0.0 (Spline|GetSplineLength (Variables|/Game/Characters/CarSTuff/SplinePathBP.SplinePathBP_C|GetSpline (Variables|Default|GetSplineRef))) _move_track) "Local") "1.000000,1.000000,1.000000")))))

(event EventBeginPlay
  (bind _returnvalue (Actor|GetActorOfClass "/Game/Characters/CarSTuff/SplinePathBP.SplinePathBP_C"))
  (Variables|Default|SetSplineRef _returnvalue)
  (CallFunction|MoveObject))

(event Collision|EventHit
  (params (MyComp :type Primitive%20Component%20Object%20Reference) (Other :type Actor%20Object%20Reference) (OtherComp :type Primitive%20Component%20Object%20Reference) (bSelfMoved :type Boolean) (HitLocation :type Vector :default "0, 0, 0") (HitNormal :type Vector :default "0, 0, 0") (NormalImpulse :type Vector :default "0, 0, 0") (Hit :type Hit%20Result%20Structure%20%28by%20ref%29))
  (bind _asbp_npc (Utilities|Casting|CastToBP_NPC Other))
  (Collision|SetCollisionEnabled (Variables|/Script/Engine.Character|GetMesh _asbp_npc) "QueryAndPhysics")
  (Collision|SetCollisionEnabled (Variables|/Script/Engine.Character|GetCapsuleComponent _asbp_npc) "NoCollision")
  (Default|ToggleTalkNotificationWidget _asbp_npc 0 false))

(fn ConstructionScript)